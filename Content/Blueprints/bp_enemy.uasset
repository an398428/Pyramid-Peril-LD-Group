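; Enemy AI character that roams random reachable points and moves to the player when PawnSensing sees or hears them.
; Reaching the player triggers a montage call gated by CanAttack.
; Separately, overlapping the player starts a looping timer that subtracts PlayerHealth while CanAttack is true.
; First-person projectiles hitting the capsule reduce EnemyHealth, and Tick destroys the actor at zero; spawn and explosion nodes are unconnected.
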(event OnSeePawn(PawnSensing)
  (params (Pawn :type Pawn%20Object%20Reference))
  (Variables|Default|SetSeesPlayer? true)
  (CallFunction|FollowPlayer))

(event OnHearNoise(PawnSensing)
  (params (Instigator :type Pawn%20Object%20Reference) (Location :type Vector%20%28by%20ref%29 :default "0, 0, 0") (Volume :type Float%20%28single-precision%29))
  (Variables|Default|SetSeesPlayer? true)
  (CallFunction|FollowPlayer))

(event OnComponentBeginOverlap(Capsule)
  (params (OverlappedComponent :type Primitive%20Component%20Object%20Reference) (OtherActor :type Actor%20Object%20Reference) (OtherComp :type Primitive%20Component%20Object%20Reference) (OtherBodyIndex :type Integer) (bFromSweep :type Boolean) (SweepResult :type Hit%20Result%20Structure%20%28by%20ref%29))
  ;[1 0.6676 0.9878] Enemy taking damage from shots
  (bind _asbp_first_person_projectile (Utilities|Casting|CastToBP_FirstPersonProjectile OtherActor))
  (Variables|Default|SetEnemyHealth (- (Variables|Default|GetEnemyHealth) 2e+01))
  (Actor|DestroyActor _asbp_first_person_projectile))

(event Custom|Random%20Roam
  (AI|AIMoveTo self (.RandomLocation (AI|Navigation|GetRandomReachablePointinRadius (Transformation|GetActorLocation) 2e+03 0 0)) 0 5.0 false
    (:OnSuccess
      (CallFunction|RandomRoam))))

(event Custom|FollowPlayer
  (Variables|Default|SetCanAttack? true)
  (if (Variables|Default|GetSeesPlayer?)
    (AI|AIMoveTo self "0, 0, 0" (Game|GetPlayerCharacter 0) 0.0 false
      (:OnSuccess
        (if (Variables|Default|GetCanAttack?)
          (Variables|Default|SetCanAttack? false)
          (bind _returnvalue (Animation|PlayAnimMontage 0 1.0 "None"))
          (Utilities|FlowControl|Delay _returnvalue)
          (Variables|Default|SetCanAttack? true))))
    (else
      (Variables|Default|SetSeesPlayer? false))))

(event Custom|ContinuousDamage
  ;[1 0.7427 0.9925] Enemy Damage to Player System
  (if (Variables|Default|GetCanAttack?)
    (bind _asbp_first_person_character (Utilities|Casting|CastToBP_FirstPersonCharacter (Game|Player|GetPlayerPawn 0)))
    (bind _output_get (Variables|/Game/FirstPerson/Blueprints/BP_FirstPersonCharacter.BP_FirstPersonCharacter_C|SetPlayerHealth _asbp_first_person_character (- (Variables|/Game/FirstPerson/Blueprints/BP_FirstPersonCharacter.BP_FirstPersonCharacter_C|GetPlayerHealth _asbp_first_person_character) 5.0)))
    (Development|PrintString (Utilities|String|ToString(Float) _output_get))))

(event EventBeginPlay
  (CallFunction|RandomRoam))

(event Collision|EventActorBeginOverlap
  (params (OtherActor :type Actor%20Object%20Reference))
  ;[1 0.7427 0.9925] Enemy Damage to Player System
  (Utilities|Casting|CastToBP_FirstPersonCharacter OtherActor)
  (Variables|Default|SetCanAttack? true)
  (Utilities|Time|SetTimerbyEvent (delegate Custom|ContinuousDamage) 0.5 true))

(event Collision|EventActorEndOverlap
  (params (OtherActor :type Actor%20Object%20Reference))
  ;[1 0.7427 0.9925] Enemy Damage to Player System
  (Utilities|Casting|CastToBP_FirstPersonCharacter OtherActor)
  (Variables|Default|SetCanAttack? false))

(event EventTick
  (params (DeltaSeconds :type Float%20%28single-precision%29))
  ;[1 0.6416 0.9669] Enemy Health & Death
  (if (<= (Variables|Default|GetEnemyHealth) 0.0)
    (Actor|DestroyActor)))

(fn ConstructionScript)