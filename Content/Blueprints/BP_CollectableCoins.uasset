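; BP_CollectableCoins is a coin pickup that spins in place and adds to the player's coin count when collected.
; Tick yaws the mesh by a fixed step each frame, so spin speed depends on frame rate.
; A PickUpRadius overlap casts the other actor's Instigator to BP_FirstPersonCharacter, increments its Coins, prints the value in gold text and destroys the coin.
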(event OnComponentBeginOverlap(PickUpRadius)
  (params (OverlappedComponent :type Primitive%20Component%20Object%20Reference) (OtherActor :type Actor%20Object%20Reference) (OtherComp :type Primitive%20Component%20Object%20Reference) (OtherBodyIndex :type Integer) (bFromSweep :type Boolean) (SweepResult :type Hit%20Result%20Structure%20%28by%20ref%29))
  (bind _asbp_first_person_character (Utilities|Casting|CastToBP_FirstPersonCharacter (Game|GetInstigator OtherActor)))
  (bind _result (Math|Integer|IncrementInt (Variables|/Game/FirstPerson/Blueprints/BP_FirstPersonCharacter.BP_FirstPersonCharacter_C|GetCoins _asbp_first_person_character))
    (:%20%20
      (Development|PrintString (Utilities|String|ToString(Integer) _result) true true "(R=1.000000,G=0.789475,B=0.000000,A=1.000000)")
      (Actor|DestroyActor))))

(event EventTick
  (params (DeltaSeconds :type Float%20%28single-precision%29))
  (Transformation|AddRelativeRotation (Variables|Default|GetMesh) (Math|Rotator|MakeRotator 0.0 0.0 3.0) false false))

(fn ConstructionScript)