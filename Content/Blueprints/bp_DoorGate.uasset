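; Gate Blueprint that opens when an overlapping first-person character has a key, and otherwise prints that it is locked.
; OpenGate toggles GateClosed and plays or reverses the RisingGate timeline, whose update sets the gate to a fixed relative X.
; CheckForKey offers a key-ID check, and UnlockDoor clears Locked, plays a sound, then calls OpenGate after it ends; neither is called within this graph.
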(event OnComponentBeginOverlap(Box)
  (params (OverlappedComponent :type Primitive%20Component%20Object%20Reference) (OtherActor :type Actor%20Object%20Reference) (OtherComp :type Primitive%20Component%20Object%20Reference) (OtherBodyIndex :type Integer) (bFromSweep :type Boolean) (SweepResult :type Hit%20Result%20Structure%20%28by%20ref%29))
  (bind _asbp_first_person_character (Utilities|Casting|CastToBP_FirstPersonCharacter OtherActor))
  (if (Variables|/Game/FirstPerson/Blueprints/BP_FirstPersonCharacter.BP_FirstPersonCharacter_C|GethasKey _asbp_first_person_character)
    (CallFunction|OpenGate)
    (else
      (Development|PrintString "Gate is locked."))))

(event Custom|OpenGate
  (if (Variables|Default|GetGateClosed?)
    (Variables|Default|SetGateClosed? false)
    (Timeline|RisingGate PlayFromStart
      (:Update
        (Transformation|SetRelativeLocation (Variables|Default|GetGate) (Math|Vector|MakeVector 1.8e+02 0.0 0.0) false false)))
    (else
      (Variables|Default|SetGateClosed? true)
      (Timeline|RisingGate Reverse))))

(event Custom|CheckForKey
  (if (Utilities|Array|ContainsItem (Variables|/Game/FirstPerson/Blueprints/BP_FirstPersonCharacter.BP_FirstPersonCharacter_C|GetKeys (Variables|Default|GetPlayerRef)) (Variables|Default|GetDoorKeyID))
    (CallFunction|OpenGate)))

(event Custom|UnlockDoor
  (bind _unlockedsound (Variables|Default|GetUnlockedSound))
  (Variables|Default|SetLocked? false)
  (Audio|PlaySoundatLocation _unlockedsound (Transformation|GetWorldLocation (Variables|Default|GetGate)) "0, 0, 0" 1.0 1.0 0.0 0 0 0 0)
  (Utilities|FlowControl|Delay (Variables|/Script/Engine.SoundBase|GetDuration _unlockedsound))
  (CallFunction|OpenGate))

(fn ConstructionScript)