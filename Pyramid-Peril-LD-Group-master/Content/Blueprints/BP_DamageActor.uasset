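; BP_DamageActor is a short-lived damage actor with a Projectile component that lowers enemy health on overlap and removes itself after a fixed lifespan.
; Actor overlap subtracts a fixed amount from bp_enemy's EnemyHealth, while the Projectile component's overlap does the same to bp_KeyEnemy's Health.
; Both paths edit the health variables directly through casts and print the new value, without destroying the actor on hit.
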(event OnComponentBeginOverlap(Projectile)
  (params (OverlappedComponent :type Primitive%20Component%20Object%20Reference) (OtherActor :type Actor%20Object%20Reference) (OtherComp :type Primitive%20Component%20Object%20Reference) (OtherBodyIndex :type Integer) (bFromSweep :type Boolean) (SweepResult :type Hit%20Result%20Structure%20%28by%20ref%29))
  (bind _asbp_key_enemy (Utilities|Casting|CastTobp_KeyEnemy OtherActor))
  (bind _output_get (Variables|/Game/Blueprints/bp_KeyEnemy.bp_KeyEnemy_C|SetHealth _asbp_key_enemy (- (Variables|/Game/Blueprints/bp_KeyEnemy.bp_KeyEnemy_C|GetHealth _asbp_key_enemy) 34.0)))
  (Development|PrintString (Utilities|String|ToString(Float) _output_get)))

(event Collision|EventActorBeginOverlap
  (params (OtherActor :type Actor%20Object%20Reference))
  (bind _asbp_enemy (Utilities|Casting|CastTobp_enemy OtherActor))
  (bind _output_get (Variables|/Game/Blueprints/bp_enemy.bp_enemy_C|SetEnemyHealth _asbp_enemy (- (Variables|/Game/Blueprints/bp_enemy.bp_enemy_C|GetEnemyHealth _asbp_enemy) 34.0)))
  (Development|PrintString (Utilities|String|ToString(Float) _output_get)))

(event EventBeginPlay
  (Actor|SetLifeSpan 5.0))

(fn ConstructionScript)